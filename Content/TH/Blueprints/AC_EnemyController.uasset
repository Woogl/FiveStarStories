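; AC_EnemyController is an AI controller that runs the BT_Guard behavior tree on possession to drive a guard enemy.
; When AI perception successfully senses an actor, it writes the AIState enum and that actor as PlayerActor to the blackboard, with no check on the actor's type.
; Lost stimuli are ignored, and the BP_Manager reference cached at BeginPlay is not used in these graphs.
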(event `self.ReceiveTick`
  (params (DeltaSeconds :type "Float (single-precision)")))

(event `self.ReceiveBeginPlay`
  (bind _returnvalue (`GameplayStatics.GetActorOfClass` "/Game/TH/Blueprints/BP_Manager.BP_Manager_C"))
  (set `self.Manager` _returnvalue))

(event `self.ReceivePossess`
  (params (PossessedPawn :type "Pawn Object Reference"))
  (`self.RunBehaviorTree` "/Game/TH/Blueprints/BT_Guard.BT_Guard"))

(event `self.AIPerception.OnTargetPerceptionUpdated`
  (params (Actor :type "Actor Object Reference") (Stimulus :type "AIStimulus Structure"))
  (bind _blackboard (`self.Blackboard`))
  (if (`.bSuccessfullySensed` (break `AIStimulus` Stimulus))
    (`BlackboardComponent.SetValueAsEnum` _blackboard (`self.AIState`) (`self.Enum`))
    (`BlackboardComponent.SetValueAsObject` _blackboard (`self.PlayerActor`) Actor)))

(fn `UserConstructionScript`)