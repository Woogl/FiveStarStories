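; BP_EnemyGuard is an enemy guard character that reacts to taking damage through its AI blackboard and BP_Manager.
; On damage it sets the AIState key, reports the hit to AI perception and calls StartAI on the manager.
; It sets the same state again when Posture is depleted and calls EnemyDie at zero Hp, though neither value changes here.
; UpdateMoveSpeed sets max walk speed; a noise report is left unconnected.
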(event `self.ReceiveAnyDamage`
  (params (Damage :type "Float (single-precision)") (DamageType :type "DamageType Object Reference") (InstigatedBy :type "Controller Object Reference") (DamageCauser :type "Actor Object Reference"))
  (bind _returnvalue (`AIBlueprintHelperLibrary.GetBlackboard` (`AIBlueprintHelperLibrary.GetAIController` self)))
  (`BlackboardComponent.SetValueAsEnum` _returnvalue (`self.AIState`) 5)
  (`AISense_Damage.ReportDamageEvent` self DamageCauser Damage (`self.K2_GetActorLocation`))
  (if (<= (`self.posture`) 0.0)
    (`BlackboardComponent.SetValueAsEnum` _returnvalue (`self.AIState`) 5))
  (bind _returnvalue_2 (`GameplayStatics.GetActorOfClass` "/Game/TH/Blueprints/BP_Manager.BP_Manager_C"))
  (`/Game/TH/Blueprints/BP_Manager.StartAI` _returnvalue_2)
  (if (<= (`self.hp`) 0.0)
    (`/Game/TH/Blueprints/BP_Manager.EnemyDie` _returnvalue_2 self)))

(fn `UpdateMoveSpeed`
  (params (NewSpeed :type "Float (double-precision)"))
  (set `CharacterMovementComponent.MaxWalkSpeed` NewSpeed (`self.CharacterMovement`)))

(fn `UserConstructionScript`)